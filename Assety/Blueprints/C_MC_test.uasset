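; Player character Blueprint for a combat game, with an ammo-based gun, knockback area skill, impulse dodge and nearest-enemy lock-on.
; A menu counter on LevelDatabaseActor selects what the action input triggers: shot, mana-costing skill or teleport to the locked enemy.
; Teleporting fires immediately, then primes a Boost spread shot.
; Timelines and Tick drive cooldowns, while Tick also updates targeting and damage UI, and destroys the character at zero HP.
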(event `InputAction|Wykonaj`
  (params (Key :type "Key Structure"))
  (bind _ammo (`self.Ammo`))
  (bind _bank_zmiennych (`self.Bank_zmiennych`))
  (bind _counter_dla_menu (`/Game/ThirdPersonCPP/Blueprints/LevelDatabaseActor.counter_dla_menu` _bank_zmiennych))
  (:`Pressed`
    ;[1 1 1] Postaw boxa po wcisnieciu, casting
    ;;[1 1 1] jezeli menu jest wlaczane
    (if (`/Game/ThirdPersonCPP/Blueprints/LevelDatabaseActor.flaga_menu` _bank_zmiennych)
      (if (== _counter_dla_menu 0)
        (bind _kod_wyjscia (`self.Glowny_atak`))
        (if _kod_wyjscia
          (if (not (== _ammo 0.0))
            (set `self.Ammo` (- _ammo 1.0))
            (bind (_direction _newtrack_0) (`Timeline|C_strzal_prawa` :!via `PlayFromStart`)
              (:`Update`
                (set `self.Cooldown_bron` _newtrack_0)))
            (else
              (`GameplayStatics.PlaySound2D` "/Game/Blueprints/dzwieki/reload.reload" 1.0 1.0 0.0 null null :!label _label)
              (bind (_direction_2 _newtrack_0_2) (`Timeline|Przeladowywanie` :!via `PlayFromStart`)
                (:`Update`
                  (set `self.Reload` _newtrack_0_2))
                (:`Finished`
                  (set `self.Ammo` 6.0))))))
        (elif (== _counter_dla_menu 1)
          (bind _kod_wyjscia_2 (`self.Skill`))
          (if _kod_wyjscia_2
            (bind (_direction_3 _newtrack_0_3) (`Timeline|Timeline_0` :!via `PlayFromStart`)
              (:`Update`
                (set `self.Skill_cooldown` _newtrack_0_3))))
          (elif (== _counter_dla_menu 2)
            (`self.Nothin_Personnel`))))
      (else
        (bind _aslevel_database_actor (cast `/Game/ThirdPersonCPP/Blueprints/LevelDatabaseActor` _bank_zmiennych))
        (set `/Game/ThirdPersonCPP/Blueprints/LevelDatabaseActor.flaga_menu` true _aslevel_database_actor)
        (`self.stworz_menu` :!label _label_2)))))

(event `InputAction|Reload`
  (params (Key :type "Key Structure"))
  (:`Pressed`
    (if (< (`self.Ammo`) 6.0)
      (goto _label))))

(event `InputAction|Menu_reverse`
  (params (Key :type "Key Structure"))
  (:`Pressed`
    (`self.decrement_counter`)))

(event `self.ReceiveBeginPlay`
  (bind _outactors (`GameplayStatics.GetAllActorsOfClass` "/Game/ThirdPersonCPP/Blueprints/LevelDatabaseActor.LevelDatabaseActor_C"))
  (set `self.Bank_zmiennych` (`|GetArrayItem` _outactors))
  (`self.Glowne_menu`)
  (goto _label_2))

(event `InputAction|PrawyPrzycisk`
  (params (Key :type "Key Structure"))
  (:`Pressed`
    (`self.wylaczanie menu`)))

(event `InputAction|Menu_input`
  (params (Key :type "Key Structure"))
  (:`Pressed`
    (`self.increment_counter` null)))

(event `InputAction|LockOn`
  (params (Key :type "Key Structure"))
  (:`Pressed`
    (if (`self.lock_on_flaga`)
      (set `self.lock_on_flaga` false)
      (else
        (set `self.lock_on_flaga` true)))))

(event `InputAction|Dodge`
  (params (Key :type "Key Structure"))
  (:`Pressed`
    (`self.Dodge_start`))
  (:`Released`
    (bind _kod_wyjscia (`self.Dodge_end`))
    (if _kod_wyjscia
      (bind (_direction _inv_czas) (`Timeline|Dodge` :!via `PlayFromStart`)
        (:`Update`
          (set `self.Invincibility frames` _inv_czas))))))

(event `self.ReceiveTick`
  (params (DeltaSeconds :type "Float (single-precision)"))
  (bind _pointlight (`self.PointLight`))
  (bind _skeletalmesh (`self.SkeletalMesh`))
  (if (> (`self.hp`) 0.0)
    ;[1 1 1] tick
    (bind _widget (`self.Damage_ui`))
    (`self.main`)
    (`self.Cooldowny` DeltaSeconds _widget)
    (`self.lockowanie_na_przeciwnika`)
    (`self.mana i cooldown`)
    (`self.reset jumpow`)
    (set `self.W_ruchu` (not (and (== (`self.GetInputAxisValue`) 0.0) (== (`self.GetInputAxisValue`) 0.0))))
    (if (`self.Boost`)
      (`SceneComponent.SetVisibility` _skeletalmesh true false)
      (`SceneComponent.SetVisibility` _pointlight true false)
      (else
        (`SceneComponent.SetVisibility` _skeletalmesh false false)
        (`SceneComponent.SetVisibility` _pointlight false false)))
    (else
      (`self.GameOver`))))

(event `self.Capsule.OnComponentBeginOverlap`
  (params (OverlappedComponent :type "PrimitiveComponent Object Reference") (OtherActor :type "Actor Object Reference") (OtherComp :type "PrimitiveComponent Object Reference") (OtherBodyIndex :type Integer) (bFromSweep :type Boolean) (SweepResult :type "HitResult Structure (by ref)"))
  (bind _asai_przeciwnik (cast `/Game/ThirdPersonCPP/Blueprints/ai_test/AI_przeciwnik` OtherActor))
  (set `/Game/ThirdPersonCPP/Blueprints/ai_test/AI_przeciwnik.W_zasiegu` true _asai_przeciwnik))

(event `InputAction|Num_1`
  (params (Key :type "Key Structure"))
  ;[1 1 1] menu pod klawiszami
  (:`Pressed`
    (bind _outactors (`GameplayStatics.GetAllActorsOfClass` "/Game/ThirdPersonCPP/Blueprints/LevelDatabaseActor.LevelDatabaseActor_C"))
    (bind _aslevel_database_actor (cast `/Game/ThirdPersonCPP/Blueprints/LevelDatabaseActor` (`|GetArrayItem` _outactors)))
    (set `/Game/ThirdPersonCPP/Blueprints/LevelDatabaseActor.counter_dla_menu` 0 _aslevel_database_actor)))

(event `self.Capsule.OnComponentEndOverlap`
  (params (OverlappedComponent :type "PrimitiveComponent Object Reference") (OtherActor :type "Actor Object Reference") (OtherComp :type "PrimitiveComponent Object Reference") (OtherBodyIndex :type Integer))
  (bind _asai_przeciwnik (cast `/Game/ThirdPersonCPP/Blueprints/ai_test/AI_przeciwnik` OtherActor))
  (set `/Game/ThirdPersonCPP/Blueprints/ai_test/AI_przeciwnik.W_zasiegu` false _asai_przeciwnik))

(event `InputAction|Num_2`
  (params (Key :type "Key Structure"))
  ;[1 1 1] menu pod klawiszami
  (:`Pressed`
    (bind _outactors (`GameplayStatics.GetAllActorsOfClass` "/Game/ThirdPersonCPP/Blueprints/LevelDatabaseActor.LevelDatabaseActor_C"))
    (bind _aslevel_database_actor (cast `/Game/ThirdPersonCPP/Blueprints/LevelDatabaseActor` (`|GetArrayItem` _outactors)))
    (set `/Game/ThirdPersonCPP/Blueprints/LevelDatabaseActor.counter_dla_menu` 1 _aslevel_database_actor)))

(event `InputAction|Num_3`
  (params (Key :type "Key Structure"))
  ;[1 1 1] menu pod klawiszami
  (:`Pressed`
    (bind _outactors (`GameplayStatics.GetAllActorsOfClass` "/Game/ThirdPersonCPP/Blueprints/LevelDatabaseActor.LevelDatabaseActor_C"))
    (bind _aslevel_database_actor (cast `/Game/ThirdPersonCPP/Blueprints/LevelDatabaseActor` (`|GetArrayItem` _outactors)))
    (set `/Game/ThirdPersonCPP/Blueprints/LevelDatabaseActor.counter_dla_menu` 2 _aslevel_database_actor)))

(fn `atak_2`)

(fn `Atak_po_podbiciu`
  (bind _returnvalue (`self.K2_GetActorRotation`))
  (bind _returnvalue_2 (`|SpawnActorFromClass` "/Game/ThirdPersonCPP/Blueprints/Instancja_Hitboxa.Instancja_Hitboxa_C" (`KismetMathLibrary.MakeTransform` (`self.K2_GetActorLocation`) _returnvalue) "AlwaysSpawn" "OverrideRootScale" null null))
  (set `/Game/ThirdPersonCPP/Blueprints/Instancja_Hitboxa.Rotator_postaci` _returnvalue _returnvalue_2)
  (set `self.Atak_Cooldown` 0.9))

(fn `Cooldowny`
  (params (czas :type "Float (double-precision)") (Widget :type "Widget Object Reference"))
  (bind _atak_cooldown (`self.Atak_Cooldown`))
  (bind _cooldown_damage (`self.Cooldown_damage`))
  (bind _invincibility_frames (`self.Invincibility frames`))
  ;[1 1 1] atak
  (if (> _atak_cooldown 0.0)
    (set `self.Atak_Cooldown` (- _atak_cooldown czas)))
  ;[1 1 1] Dodge
  (if (> _invincibility_frames 0.0)
    (set `self.Invincibility frames` (- _invincibility_frames czas)))
  (if (> _cooldown_damage 0.0)
    (bind _output_get (set `self.Cooldown_damage` (- _cooldown_damage czas)))
    (set `self.Damage` false)
    (if (<= _output_get 0.0)
      (bind _foundwidgets (`WidgetBlueprintLibrary.GetAllWidgetsOfClass` "/Game/UI/Damage.Damage_C"))
      (for _array_element _foundwidgets
        (`Widget.RemoveFromParent` _array_element))))
  (return))

(fn `DAB`)

(fn `DABB_Refresh`
  (bind _returnvalue (`PrimitiveComponent.GetPhysicsLinearVelocity` (`self.CapsuleComponent`) "None"))
  (if (== (.z _returnvalue) 0.0)
    (add `self.OnReachedJumpApex` (`|CreateDelegate` :!event `DAB`))
    (set `CharacterMovementComponent.bNotifyApex` true (`self.CharacterMovement`))))

(fn `Damage_ui`
  (returns (Widget :type "Widget Object Reference"))
  (if (`self.Damage`)
    (bind _returnvalue (`|CreateWidget` "/Game/UI/Damage.Damage_C"))
    (`UserWidget.AddToViewport` _returnvalue 0)
    (set `self.Cooldown_damage` 0.1)
    (return _returnvalue)
    (else
      (bind _returnvalue_2 (`|CreateWidget` "/Game/UI/Damage.Damage_C"))
      (return _returnvalue_2))))

(fn `decrement_counter`
  ;[1 1 1] odejmij wartosc countera (modyfikowalne)
  (bind _outactors (`GameplayStatics.GetAllActorsOfClass` "/Game/ThirdPersonCPP/Blueprints/LevelDatabaseActor.LevelDatabaseActor_C"))
  (bind _output (`|GetArrayItem` _outactors))
  (bind _aslevel_database_actor (cast `/Game/ThirdPersonCPP/Blueprints/LevelDatabaseActor` _output))
  (set `/Game/ThirdPersonCPP/Blueprints/LevelDatabaseActor.counter_dla_menu` (mod (+ (`/Game/ThirdPersonCPP/Blueprints/LevelDatabaseActor.counter_dla_menu` _output) 2) 3) _aslevel_database_actor))

(fn `Dodge_end`
  (returns (`kod wyjscia` :type Boolean))
  (bind _dodge_speed (`self.dodge_speed`))
  (bind _pozycja_startowa_dodge (`self.Pozycja_startowa_dodge`))
  (bind _returnvalue (/ (`self.dodge_speed`) 3.0))
  (bind _y (.y (- (`self.Pozycja_startowa_dodge`) (`self.K2_GetActorLocation` (`GameplayStatics.GetPlayerCharacter` 0)))))
  (bind _y_2 (.y (- _pozycja_startowa_dodge (`self.K2_GetActorLocation` (`GameplayStatics.GetPlayerCharacter` 0)))))
  (bind _returnvalue_2 (`KismetMathLibrary.DegAtan` (/ (.x (- _pozycja_startowa_dodge (`self.K2_GetActorLocation` (`GameplayStatics.GetPlayerCharacter` 0)))) _y_2)))
  (bind _returnvalue_3 (`KismetMathLibrary.DegAtan` (/ (.x (- (`self.Pozycja_startowa_dodge`) (`self.K2_GetActorLocation` (`GameplayStatics.GetPlayerCharacter` 0)))) _y)))
  (bind _returnvalue_4 (* (`KismetMathLibrary.DegCos` _returnvalue_3) _returnvalue))
  (bind _returnvalue_5 (* (`KismetMathLibrary.DegSin` _returnvalue_3) _returnvalue))
  (bind _returnvalue_6 (* (`KismetMathLibrary.DegSin` _returnvalue_2) _dodge_speed))
  (bind _returnvalue_7 (* (`KismetMathLibrary.DegCos` _returnvalue_2) _dodge_speed))
  (if (== (`self.Invincibility frames`) 0.0)
    (if (!= _pozycja_startowa_dodge (0.0 0.0 0.0) :`ErrorTolerance` 0.0)
      (set `self.Invincibility frames` 0.2)
      (if (`NavMovementComponent.IsMovingOnGround` (`self.CharacterMovement`))
        (if (> _y_2 0.0)
          (`CharacterMovementComponent.AddImpulse` (`self.CharacterMovement`) (`KismetMathLibrary.MakeVector` (* _returnvalue_6 -1.0) (* _returnvalue_7 -1.0)) true)
          (else
            (`CharacterMovementComponent.AddImpulse` (`self.CharacterMovement`) (`KismetMathLibrary.MakeVector` _returnvalue_6 _returnvalue_7) true)))
        (set `self.Pozycja_startowa_dodge` (0.0 0.0 0.0))
        (return true)
        (else
          (if (> _y 0.0)
            (`CharacterMovementComponent.AddImpulse` (`self.CharacterMovement`) (`KismetMathLibrary.MakeVector` (* _returnvalue_5 -1.0) (* _returnvalue_4 -1.0)) true)
            (else
              (`CharacterMovementComponent.AddImpulse` (`self.CharacterMovement`) (`KismetMathLibrary.MakeVector` _returnvalue_5 _returnvalue_4) true)))
          (set `self.Pozycja_startowa_dodge` (0.0 0.0 0.0))
          (return true))))
    (else
      (return false))))

(fn `Dodge_start`
  (if true
    (set `self.Pozycja_startowa_dodge` (`self.K2_GetActorLocation` (`GameplayStatics.GetPlayerCharacter` 0)))
    (else
      (set `self.Pozycja_startowa_dodge` (0.0 0.0 0.0)))))

(fn `GameOver`
  (`WidgetLayoutLibrary.RemoveAllWidgets`)
  (`self.K2_DestroyActor`))

(fn `Glowne_menu`
  (bind _returnvalue (`|CreateWidget` "/Game/UI/HUD.HUD_C"))
  (`UserWidget.AddToViewport` _returnvalue 0))

(fn `Glowny_atak`
  (returns (`Kod wyjscia` :type Boolean))
  (bind _returnvalue (`self.K2_GetActorRotation`))
  (if (and (== (`self.Cooldown_bron`) 0.0) (== (`self.Reload`) 0.0))
    (if (> (`self.Ammo`) 0.0)
      (if (`self.Boost`)
        (`GameplayStatics.PlaySound2D` "/Game/Blueprints/dzwieki/shoot.shoot" 1.0 1.0 0.0 null null)
        (`GameplayStatics.PlaySound2D` "/Game/Blueprints/dzwieki/silny_strzal.silny_strzal" 1.0 1.0 0.0 null null)
        (set `self.Boost` false)
        (for _index (range 6)
          (bind _returnvalue_2 (`KismetMathLibrary.MakeRotator` (.roll (`self.K2_GetActorRotation`)) (.pitch (`self.K2_GetActorRotation`)) (+ (- (.yaw (`self.K2_GetActorRotation`)) 15.0) (* _index 5.0))))
          (bind _returnvalue_3 (`|SpawnActorFromClass` "/Game/ThirdPersonCPP/Blueprints/strzala_gracza.strzala_gracza_C" (`KismetMathLibrary.MakeTransform` (`SceneComponent.K2_GetComponentLocation` (`self.Bron`)) _returnvalue_2) "AlwaysSpawn" "OverrideRootScale" null null))
          (set `/Game/ThirdPersonCPP/Blueprints/strzala_gracza.Rotator_postaci` _returnvalue_2 _returnvalue_3))
        (else
          (`GameplayStatics.PlaySound2D` "/Game/Blueprints/dzwieki/shoot.shoot" 1.0 1.0 0.0 null null)
          (bind _returnvalue_4 (`|SpawnActorFromClass` "/Game/ThirdPersonCPP/Blueprints/strzala_gracza.strzala_gracza_C" (`KismetMathLibrary.MakeTransform` (`SceneComponent.K2_GetComponentLocation` (`self.Bron`)) _returnvalue) "AlwaysSpawn" "OverrideRootScale" null null))
          (if (`self.W_ruchu`)
            ;[1 1 1] recoil
            (set `/Game/ThirdPersonCPP/Blueprints/strzala_gracza.Wartosc_losowa` 0.0 _returnvalue_4)
            (else
              (set `/Game/ThirdPersonCPP/Blueprints/strzala_gracza.Wartosc_losowa` 0.0 _returnvalue_4)))
          (set `/Game/ThirdPersonCPP/Blueprints/strzala_gracza.Rotator_postaci` _returnvalue _returnvalue_4)
          ;[1 1 1] lewa
          (return true)))
      (else
        (return true)))
    (else
      (return false))))

(fn `increment_counter`
  (params (NewParam :type "Actor Object Reference"))
  ;[1 1 1] dodaj wartosc countera (modyfikowalne)
  (bind _outactors (`GameplayStatics.GetAllActorsOfClass` "/Game/ThirdPersonCPP/Blueprints/LevelDatabaseActor.LevelDatabaseActor_C"))
  (bind _output (`|GetArrayItem` _outactors))
  (bind _result (`/Engine/EditorBlueprintResources/StandardMacros.IncrementInt` (`/Game/ThirdPersonCPP/Blueprints/LevelDatabaseActor.counter_dla_menu` _output))
    (:`  `
      (bind _aslevel_database_actor (cast `/Game/ThirdPersonCPP/Blueprints/LevelDatabaseActor` _output))
      (set `/Game/ThirdPersonCPP/Blueprints/LevelDatabaseActor.counter_dla_menu` (mod _result 3) _aslevel_database_actor))))

(fn `lockowanie_na_przeciwnika`
  (set `self.w_co_celuje` 0)
  (bind _outactors (`GameplayStatics.GetAllActorsOfClass` "/Game/ThirdPersonCPP/Blueprints/ai_test/AI_przeciwnik.AI_przeciwnik_C"))
  (for _array_element _outactors
    (set `/Game/ThirdPersonCPP/Blueprints/ai_test/AI_przeciwnik.Celowany` false _array_element)
    (`KismetArrayLibrary.Array_Add` (`self.lista_przeciwnikow`) (`self.GetDistanceTo` _array_element)))
  (bind _output_get (set `self.w_co_celuje` (`KismetMathLibrary.MinOfFloatArray` (`self.lista_przeciwnikow`))))
  (bind _output (`|GetArrayItem` _outactors _output_get))
  (bind _asai_przeciwnik (cast `/Game/ThirdPersonCPP/Blueprints/ai_test/AI_przeciwnik` _output))
  (if (`self.lock_on_flaga`)
    (bind _returnvalue (`self.K2_GetActorLocation` _output))
    (set `self.lokacja_przeciwnika` _returnvalue)
    (set `/Game/ThirdPersonCPP/Blueprints/ai_test/AI_przeciwnik.Celowany` true _asai_przeciwnik)
    (bind _x (.x (- _returnvalue (`self.K2_GetActorLocation` (`GameplayStatics.GetPlayerCharacter` 0)))))
    (if (< _x 0.0)
      (bind _returnvalue_2 (`KismetMathLibrary.DegAtan` (/ (.y (- _returnvalue (`self.K2_GetActorLocation` (`GameplayStatics.GetPlayerCharacter` 0)))) _x)))
      (`self.K2_SetActorRotation` (`KismetMathLibrary.MakeRotator` 0.0 0.0 (+ _returnvalue_2 180.0)))
      (else
        (`self.K2_SetActorRotation` (`KismetMathLibrary.MakeRotator` 0.0 0.0 _returnvalue_2))))
    (set `self.lista_przeciwnikow` (`self.pusty`))
    (else
      (set `/Game/ThirdPersonCPP/Blueprints/ai_test/AI_przeciwnik.Celowany` false _asai_przeciwnik)
      (set `self.lista_przeciwnikow` (`self.pusty`)))))

(fn `main`
  (bind _outactors (`GameplayStatics.GetAllActorsOfClass` "/Game/ThirdPersonCPP/Blueprints/LevelDatabaseActor.LevelDatabaseActor_C"))
  (bind _output (`|GetArrayItem` _outactors))
  (if (`/Game/ThirdPersonCPP/Blueprints/LevelDatabaseActor.flaga_menu` _output)
    (bind _outactors_2 (`GameplayStatics.GetAllActorsOfClass` "/Game/ThirdPersonCPP/Blueprints/LevelDatabaseActor.LevelDatabaseActor_C"))
    (if (== (`/Game/ThirdPersonCPP/Blueprints/LevelDatabaseActor.counter_dla_menu` (`|GetArrayItem` _outactors_2)) 0)
      (`self.obrot wskaznika`))
    (else
      ;[1 1 1] jezeli menu jest wylaczone wylacz wskaznik
      (bind _aslevel_database_actor (cast `/Game/ThirdPersonCPP/Blueprints/LevelDatabaseActor` _output))
      (set `/Game/ThirdPersonCPP/Blueprints/LevelDatabaseActor.counter_dla_menu` 4 _aslevel_database_actor)
      (bind _outactors_3 (`GameplayStatics.GetAllActorsOfClass` "/Game/ThirdPersonCPP/Blueprints/Hitboxeu.Hitboxeu_C"))
      (`self.K2_DestroyActor` _outactors_3))))

(fn `mana i cooldown`
  (bind _tp_cooldown (`self.Tp_cooldown`))
  (if (!= _tp_cooldown 0.0)
    (set `self.Tp_cooldown` (- _tp_cooldown 0.08)))
  (if (<= (`self.Mana`) 100.0)
    (set `self.Mana` (+ (`self.Mana`) 0.0)))
  (return))

(fn `menu`)

(fn `Nothin_Personnel`
  (bind _ammo (`self.Ammo`))
  (bind _outactors (`GameplayStatics.GetAllActorsOfClass` "/Game/ThirdPersonCPP/Blueprints/ai_test/AI_przeciwnik.AI_przeciwnik_C"))
  (if (and (> (`KismetArrayLibrary.Array_Length` _outactors) 0) (<= (`self.Tp_cooldown`) 0.0))
    (if (`self.lock_on_flaga`)
      (set `self.Tp_cooldown` 10.0)
      (bind _outactors_2 (`GameplayStatics.GetAllActorsOfClass` "/Game/ThirdPersonCPP/Blueprints/ai_test/AI_przeciwnik.AI_przeciwnik_C"))
      (bind _output (`|GetArrayItem` _outactors_2 (`self.w_co_celuje`)))
      (`self.K2_SetActorTransform` (`KismetMathLibrary.MakeTransform` (`KismetMathLibrary.MakeVector` (+ (.x (`SceneComponent.K2_GetComponentLocation` (`/Game/ThirdPersonCPP/Blueprints/ai_test/AI_przeciwnik.teleport_spot` _output))) 50.0) (+ (.y (`SceneComponent.K2_GetComponentLocation` (`/Game/ThirdPersonCPP/Blueprints/ai_test/AI_przeciwnik.teleport_spot` _output))) 50.0) (.z (`SceneComponent.K2_GetComponentLocation` (`/Game/ThirdPersonCPP/Blueprints/ai_test/AI_przeciwnik.teleport_spot` _output)))) (`self.K2_GetActorRotation` _output) (.scale (`self.GetTransform` (`GameplayStatics.GetPlayerCharacter` 0)))))
      (set `/Game/ThirdPersonCPP/Blueprints/LevelDatabaseActor.counter_dla_menu` 0 (`self.Bank_zmiennych`))
      (`self.Glowny_atak`)
      (`GameplayStatics.PlaySound2D` "/Game/Blueprints/dzwieki/DBZ_Instant_Transmission_Sound_effect.DBZ_Instant_Transmission_Sound_effect" 1.0 1.0 0.0 null null)
      (set `self.Boost` true)
      (if (< _ammo 6.0)
        (set `self.Ammo` (+ _ammo 1.0)))
      (return))))

(fn `obrot wskaznika`
  ;[1 1 1] obraca wskaznik
  (bind _outactors (`GameplayStatics.GetAllActorsOfClass` "/Game/ThirdPersonCPP/Blueprints/Hitboxeu.Hitboxeu_C"))
  (if (> (`KismetArrayLibrary.Array_Length` _outactors) 0)
    (`self.K2_SetActorTransform` (`|GetArrayItem` _outactors) (`KismetMathLibrary.MakeTransform` (`self.K2_GetActorLocation`) (`self.K2_GetActorRotation`)) false false)))

(fn `Pokazuje_atak`)

(fn `reset jumpow`
  (if (`NavMovementComponent.IsMovingOnGround` (`self.CharacterMovement`))
    (set `self.JumpMaxCount` 2))
  (return))

(fn `Skill`
  (returns (kod_wyjscia :type Boolean))
  (locals (Wartosc :type "Float (double-precision)" :default 1000.0))
  (bind _returnvalue (`GameplayStatics.GetPlayerCharacter` 0))
  (bind _mana (`self.Mana`))
  (bind _returnvalue_2 (* (`local.Wartosc`) -1.0))
  (if (and (== (`self.Skill_cooldown`) 0.0) (>= _mana 20.0))
    (set `self.Mana` (- _mana 20.0))
    (bind _outactors (`GameplayStatics.GetAllActorsOfClass` "/Game/ThirdPersonCPP/Blueprints/ai_test/AI_przeciwnik.AI_przeciwnik_C"))
    (for _array_element _outactors
      (if (< (`self.GetDistanceTo` _returnvalue _array_element) 700.0)
        (set `/Game/ThirdPersonCPP/Blueprints/ai_test/AI_przeciwnik.Zycie` (- (`/Game/ThirdPersonCPP/Blueprints/ai_test/AI_przeciwnik.Zycie` _array_element) 30.0) _array_element)
        (bind _returnvalue_3 (- (.x (`self.K2_GetActorLocation` _returnvalue)) (.x (`self.K2_GetActorLocation` _array_element))))
        (bind _returnvalue_4 (- (.y (`self.K2_GetActorLocation` _returnvalue)) (.y (`self.K2_GetActorLocation` _array_element))))
        (bind _returnvalue_5 (+ (`KismetMathLibrary.Abs` _returnvalue_3) (`KismetMathLibrary.Abs` _returnvalue_4)))
        (`CharacterMovementComponent.AddImpulse` (`Character.CharacterMovement` _array_element) (`KismetMathLibrary.MakeVector` (* (/ _returnvalue_3 _returnvalue_5) _returnvalue_2) (* (/ _returnvalue_4 _returnvalue_5) _returnvalue_2) 2000.0) true)
        (return true)))
    (else
      (return false))))

(fn `stworz_menu`
  ;[1 1 1] tworzy menu
  (bind _outactors (`GameplayStatics.GetAllActorsOfClass` "/Game/ThirdPersonCPP/Blueprints/LevelDatabaseActor.LevelDatabaseActor_C"))
  (if (`/Game/ThirdPersonCPP/Blueprints/LevelDatabaseActor.flaga_menu` (`|GetArrayItem` _outactors))
    (bind _returnvalue (`|CreateWidget` "/Game/UI/menu.menu_C"))
    (`UserWidget.AddToViewport` _returnvalue 0)))

(fn `Teleportacja_combo`
  (bind _outactors (`GameplayStatics.GetAllActorsOfClass` "/Game/ThirdPersonCPP/Blueprints/ai_test/AI_przeciwnik.AI_przeciwnik_C"))
  (bind _output (`|GetArrayItem` _outactors (`self.w_co_celuje`)))
  (`self.K2_SetActorTransform` (`KismetMathLibrary.MakeTransform` (`KismetMathLibrary.MakeVector` (+ (.x (`SceneComponent.K2_GetComponentLocation` (`/Game/ThirdPersonCPP/Blueprints/ai_test/AI_przeciwnik.teleport_spot` _output))) 50.0) (+ (.y (`SceneComponent.K2_GetComponentLocation` (`/Game/ThirdPersonCPP/Blueprints/ai_test/AI_przeciwnik.teleport_spot` _output))) 50.0) (.z (`SceneComponent.K2_GetComponentLocation` (`/Game/ThirdPersonCPP/Blueprints/ai_test/AI_przeciwnik.teleport_spot` _output)))) (`self.K2_GetActorRotation` _output) (.scale (`self.GetTransform` (`GameplayStatics.GetPlayerCharacter` 0))))))

(fn `UserConstructionScript`
  (`self.Glowne_menu`)
  (add `self.OnReachedJumpApex` (`|CreateDelegate` :!event `DABB_Refresh`))
  (set `CharacterMovementComponent.bNotifyApex` true (`self.CharacterMovement`)))

(fn `wylaczanie menu`
  ;[1 1 1] wylacz menu
  (`WidgetLayoutLibrary.RemoveAllWidgets`)
  (bind _outactors (`GameplayStatics.GetAllActorsOfClass` "/Game/ThirdPersonCPP/Blueprints/LevelDatabaseActor.LevelDatabaseActor_C"))
  (bind _aslevel_database_actor (cast `/Game/ThirdPersonCPP/Blueprints/LevelDatabaseActor` (`|GetArrayItem` _outactors)))
  (set `/Game/ThirdPersonCPP/Blueprints/LevelDatabaseActor.flaga_menu` false _aslevel_database_actor)
  (bind _returnvalue (`|CreateWidget` "/Game/UI/HUD.HUD_C"))
  (`UserWidget.AddToViewport` _returnvalue 0))